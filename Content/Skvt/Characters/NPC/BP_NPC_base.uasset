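; Base NPC character that takes damage, responds to player interactions and dies into a ragdoll.
; Damage feeds the health component and plays a hit montage; its death signal enables mesh physics, disables movement and destroys the actor after a delay.
; Primary interaction briefly shows hello text.
; Secondary interaction is a one-time neck-break takedown, zeroing health and playing paired NPC and player animations before restoring the player's Animation Blueprint.
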(event SignalPrimaryInteraction(InteractionComponent)
  (Rendering|SetVisibility (Variables|Default|GetHelloText) true false)
  (Utilities|FlowControl|Delay 3.0)
  (Rendering|SetVisibility (Variables|Default|GetHelloText) false false))

(event SignalCharacterDeath(SkvtHealthComponent)
  (CallFunction|TriggerDeath))

(event SignalSecondaryInteraction(InteractionComponent)
  (bind _returnvalue (Game|GetPlayerController 0))
  (bind _returnvalue_2 (Pawn|GetControlledPawn _returnvalue))
  (bind _asbp_skvt_base_char (Utilities|Casting|CastToBP_SkvtBaseChar _returnvalue_2))
  (bind _mesh (Variables|/Script/Engine.Character|GetMesh _asbp_skvt_base_char))
  (Utilities|FlowControl|DoOnce false
    (:Completed
      (Utilities|FlowControl|Sequence
        (:then_0
          ;[1 1 1] Hit animation of NPC character
          (Components|Animation|PlayAnimation (Variables|Character|GetMesh) "/Game/Skvt/Characters/Animations/Attacks/Hit_BreakNeck.Hit_BreakNeck" false)
          (Variables|/Game/Skvt/Systems/Health/SkvtHealthComponent.SkvtHealthComponent_C|SetHealth (Variables|Default|GetSkvtHealthComponent) 0.0))
        (:then_1
          ;[1 1 1] Break neck animation of player
          (Components|Animation|PlayAnimation _mesh "/Game/Skvt/Characters/Animations/Attacks/Att_BreakNeck.Att_BreakNeck" false)
          (Utilities|FlowControl|Delay (Variables|/Script/Engine.AnimSequenceBase|GetSequenceLength (Variables|Default|Getatt_breakNeckAnimation)))
          (Components|Animation|SetAnimationMode _mesh "AnimationBlueprint"))))))

(event EventBeginPlay)

(event Collision|EventActorBeginOverlap
  (params (OtherActor :type Actor%20Object%20Reference)))

(event EventTick
  (params (DeltaSeconds :type Float%20%28single-precision%29)))

(event Game|Damage|EventAnyDamage
  (params (Damage :type Float%20%28single-precision%29) (DamageType :type Damage%20Type%20Object%20Reference) (InstigatedBy :type Controller%20Object%20Reference) (DamageCauser :type Actor%20Object%20Reference))
  (Default|ProcessDamage (Variables|Default|GetSkvtHealthComponent) Damage)
  (Animation|PlayAnimMontage "/Game/Skvt/Characters/Animations/Attacks/AM_Hit_punch.AM_Hit_punch" 1.0 "None"))

(fn ConstructionScript)

(fn TriggerDeath
  (Physics|SetSimulatePhysics (Variables|Character|GetMesh) true)
  (Pawn|Components|CharacterMovement|DisableMovement (Variables|Character|GetCharacterMovement))
  (Utilities|Time|SetTimerbyFunctionName 0 "FinalizeDeath" 3.0))

(fn FinalizeDeath
  (Actor|DestroyActor))